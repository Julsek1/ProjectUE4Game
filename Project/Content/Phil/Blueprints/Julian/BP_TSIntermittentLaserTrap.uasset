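; Intermittent laser trap that alternates between off and on while hurting the player.
; Tick drives both loops through Delay nodes, switching the laser every two seconds and checking for damage on a short interval.
; Any actor overlap sets a damage flag, which makes the check call GetHit on player 0's ParentPlayer character.
; The damage check reads only that flag, not the laser state.
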(event EventBeginPlay)

(event Collision|EventActorBeginOverlap
  (params (OtherActor :type Actor%20Object%20Reference))
  (Variables|Default|SetShouldDamage true))

(event EventTick
  (params (DeltaSeconds :type Float%20%28single-precision%29))
  (Utilities|FlowControl|Sequence
    (:then_0
      (Utilities|FlowControl|Delay 2.0)
      (Class|LaserTrap|DeactivateLaser)
      (Utilities|FlowControl|Delay 2.0)
      (Class|LaserTrap|ActivateLaser))
    (:then_1
      (Utilities|FlowControl|Delay 0.1)
      (if (Variables|Default|GetShouldDamage)
        (bind _asparent_player (Utilities|Casting|CastToParentPlayer (Game|GetPlayerCharacter 0)))
        (Class|ParentPlayer|GetHit _asparent_player 0.01)))))

(event Collision|EventActorEndOverlap
  (params (OtherActor :type Actor%20Object%20Reference))
  (Variables|Default|SetShouldDamage false))

(fn ConstructionScript)