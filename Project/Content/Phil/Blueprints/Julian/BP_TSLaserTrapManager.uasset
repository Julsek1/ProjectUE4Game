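; BP_TSLaserTrapManager is a laser trap manager that alternates two groups of lasers on a repeating cycle.
; On BeginPlay it deactivates every laser in LaserCycle2, leaves LaserCycle1 in its initial state, and starts a looping timer at CycleTime.
; Each timer tick calls SwapLasers, which flips each laser in both groups based on its own IsActive state, so the groups alternate only if LaserCycle1 starts active.
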(event EventBeginPlay
  (for _array_element (Variables|Default|GetLaserCycle1)
    _)
  (for _array_element_2 (Variables|Default|GetLaserCycle2)
    (Default|Deactivate _array_element_2))
  (Utilities|Time|SetTimerbyFunctionName 0 "SwapLasers" (Variables|Default|GetCycleTime) true))

(event Collision|EventActorBeginOverlap
  (params (OtherActor :type Actor%20Object%20Reference)))

(event EventTick
  (params (DeltaSeconds :type Float%20%28single-precision%29)))

(fn ConstructionScript)

(fn SwapLasers
  (for _array_element (Variables|Default|GetLaserCycle1)
    (if (Variables|/Game/Phil/Blueprints/Julian/BP_TSIntermittentLaserTrap.BP_TSIntermittentLaserTrap_C|GetIsActive _array_element)
      (Default|Deactivate _array_element)
      (else
        (Default|Activate _array_element))))
  (for _array_element_2 (Variables|Default|GetLaserCycle2)
    (if (Variables|/Game/Phil/Blueprints/Julian/BP_TSIntermittentLaserTrap.BP_TSIntermittentLaserTrap_C|GetIsActive _array_element_2)
      (Default|Deactivate _array_element_2)
      (else
        (Default|Activate _array_element_2)))))