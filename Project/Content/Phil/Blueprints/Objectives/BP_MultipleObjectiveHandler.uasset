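; BP_MultipleObjectiveHandler is an actor that manages a group of objectives where taking any one removes the rest.
; Every Tick it scans the Objectives array for an invalid entry, treating a destroyed objective as taken.
; Once one is found, it destroys all remaining valid objectives and then itself.
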(event EventBeginPlay)

(event Collision|EventActorBeginOverlap
  (params (OtherActor :type Actor%20Object%20Reference)))

(event EventTick
  (params (DeltaSeconds :type Float%20%28single-precision%29))
  (bind _array_element (Utilities|Array|ForEachLoopwithBreak (Variables|Default|GetObjectives) :!label _label)
    (:LoopBody
      (Utilities|IsValid _array_element
        (:Is%20Not%20Valid
          (Variables|Default|SetObjectiveTaken true)
          (goto _label Break))))
    (:Completed
      (if (Variables|Default|GetObjectiveTaken)
        (for _array_element_2 (Variables|Default|GetObjectives)
          (Utilities|IsValid _array_element_2
            (:Is%20Valid
              (Actor|DestroyActor _array_element_2))))
        (Actor|DestroyActor)))))

(fn ConstructionScript)