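; Blue miniboss enemy with a child-actor weapon, cached on BeginPlay as its Sniper reference.
; BeginPlay also sets the player character as owner and tints the minimap icon and damage shield with the enemy's Color.
; Tick shows the shield only at full damage resistance while alive; once dead, it hides the icon and weapon and disables capsule collision.
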(event EventBeginPlay
  (Actor|SetOwner (Game|GetPlayerCharacter 0))
  (Sprite|SetSpriteColor (Variables|Default|GetMinimapIcon) (Math|Conversions|ToLinearColor(Color) (Variables|Default|GetColor)))
  (Effects|Components|ParticleSystem|SetColorParameter (Variables|Default|GetDamageShield) "ShieldColor" (Math|Conversions|ToLinearColor(Color) (Variables|Default|GetColor)))
  (bind _asbp_miniboss_blue_weapon (Utilities|Casting|CastToBP_MinibossBlueWeapon (Variables|/Script/Engine.ChildActorComponent|GetChildActor (Variables|Default|GetWeapon))))
  (Variables|Default|SetSniper _asbp_miniboss_blue_weapon))

(event Collision|EventActorBeginOverlap
  (params (OtherActor :type Actor%20Object%20Reference)))

(event EventTick
  (params (DeltaSeconds :type Float%20%28single-precision%29))
  (if (Variables|Default|GetbIsDead)
    (Rendering|SetVisibility (Variables|Default|GetMinimapIcon) false false)
    (Rendering|SetVisibility (Variables|Default|GetWeapon) false false)
    (Collision|SetCollisionEnabled (Variables|Default|GetCapsuleComponent) "NoCollision")
    (else
      (Rendering|SetVisibility (Variables|Default|GetDamageShield) (== (Variables|Default|GetDamageResistance) 1.0) false))))

(fn ConstructionScript)