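; Red miniboss enemy that carries a rocket launcher as a child-actor weapon and shows a colored damage shield.
; BeginPlay sets the player character as owner, tints the minimap icon and shield from its Color, and caches the weapon as RocketLauncher.
; Tick shows the shield only while DamageResistance equals 1.0.
; Once dead, Tick instead hides the minimap icon and weapon and disables capsule collision.
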(event EventBeginPlay
  (bind _damageshield (Variables|Default|GetDamageShield))
  (Actor|SetOwner (Game|GetPlayerCharacter 0))
  (Sprite|SetSpriteColor (Variables|Default|GetMinimapIcon) (Math|Conversions|ToLinearColor(Color) (Variables|Default|GetColor)))
  (bind _asminiboss_red_weapon (Utilities|Casting|CastToMinibossRedWeapon (Variables|/Script/Engine.ChildActorComponent|GetChildActor (Variables|Default|GetWeapon))))
  (Variables|Default|SetRocketLauncher _asminiboss_red_weapon)
  (Rendering|Material|SetMaterial _damageshield 0 (Rendering|Material|GetMaterial (Variables|Default|GetDamageShield) 0))
  (Effects|Components|ParticleSystem|SetColorParameter _damageshield "ShieldColor" (Math|Conversions|ToLinearColor(Color) (Variables|Default|GetColor))))

(event Collision|EventActorBeginOverlap
  (params (OtherActor :type Actor%20Object%20Reference)))

(event EventTick
  (params (DeltaSeconds :type Float%20%28single-precision%29))
  (if (Variables|Default|GetbIsDead)
    (Rendering|SetVisibility (Variables|Default|GetMinimapIcon) false false)
    (Rendering|SetVisibility (Variables|Default|GetWeapon) false false)
    (Collision|SetCollisionEnabled (Variables|Default|GetCapsuleComponent) "NoCollision")
    (else
      (Rendering|SetVisibility (Variables|Default|GetDamageShield) (== (Variables|Default|GetDamageResistance) 1.0) false))))

(fn ConstructionScript)