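; BP_ShieldGenerator is a miniboss shield generator that displays a protective shield while it cannot take damage.
; On BeginPlay it reapplies the DamageShield material and tints its ShieldColor parameter with the linked Miniboss's color.
; Every Tick it sets the shield's visibility to the inverse of CanTakeDamage.
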(event EventBeginPlay
  (bind _damageshield (Variables|Default|GetDamageShield))
  (Rendering|Material|SetMaterial _damageshield 0 (Rendering|Material|GetMaterial (Variables|Default|GetDamageShield) 0))
  (Effects|Components|ParticleSystem|SetColorParameter _damageshield "ShieldColor" (Math|Conversions|ToLinearColor(Color) (Variables|/Script/Project.Miniboss|GetColor (Variables|Default|GetMiniboss)))))

(event Collision|EventActorBeginOverlap
  (params (OtherActor :type Actor%20Object%20Reference)))

(event EventTick
  (params (DeltaSeconds :type Float%20%28single-precision%29))
  (Rendering|SetVisibility (Variables|Default|GetDamageShield) (not (Variables|Default|GetbCanTakeDamage)) false))

(fn ConstructionScript)