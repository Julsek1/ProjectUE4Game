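; BP_MinibossGreen is a miniboss enemy with a minimap icon and a color-tinted damage shield.
; On BeginPlay it sets the player character as its owner and applies its Color to the icon and shield.
; Each Tick, it shows the shield only at full DamageResistance while alive, or hides the icon and disables capsule collision once dead.
; An unconnected node for hiding the weapon never runs.
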(event EventBeginPlay
  (Actor|SetOwner (Game|GetPlayerCharacter 0))
  (Sprite|SetSpriteColor (Variables|Default|GetMinimapIcon) (Math|Conversions|ToLinearColor(Color) (Variables|Default|GetColor)))
  (Rendering|Material|SetMaterial (Variables|Default|GetDamageShield) 0 (Rendering|Material|GetMaterial (Variables|Default|GetDamageShield) 0))
  (Effects|Components|ParticleSystem|SetColorParameter (Variables|Default|GetDamageShield) "ShieldColor" (Math|Conversions|ToLinearColor(Color) (Variables|Default|GetColor))))

(event Collision|EventActorBeginOverlap
  (params (OtherActor :type Actor%20Object%20Reference)))

(event EventTick
  (params (DeltaSeconds :type Float%20%28single-precision%29))
  (if (Variables|Default|GetbIsDead)
    (Rendering|SetVisibility (Variables|Default|GetMinimapIcon) false false)
    (Collision|SetCollisionEnabled (Variables|Default|GetCapsuleComponent) "NoCollision")
    (else
      (Rendering|SetVisibility (Variables|Default|GetDamageShield) (== (Variables|Default|GetDamageResistance) 1.0) false))))

(fn ConstructionScript)