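; BP_MinibossGreenClone is the clone enemy for the green miniboss, armed with a shotgun.
; On BeginPlay it tints its minimap icon with its Color and caches the Weapon child actor as a MinibossGreenWeapon in Shotgun.
; Tick polls IsDead and, once true, hides the minimap icon and weapon and disables capsule collision on every frame.
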(event EventBeginPlay
  (Sprite|SetSpriteColor (Variables|Default|GetMinimapIcon) (Math|Conversions|ToLinearColor(Color) (Variables|Default|GetColor)))
  (bind _asminiboss_green_weapon (Utilities|Casting|CastToMinibossGreenWeapon (Variables|/Script/Engine.ChildActorComponent|GetChildActor (Variables|Default|GetWeapon))))
  (Variables|Default|SetShotgun _asminiboss_green_weapon))

(event Collision|EventActorBeginOverlap
  (params (OtherActor :type Actor%20Object%20Reference)))

(event EventTick
  (params (DeltaSeconds :type Float%20%28single-precision%29))
  (if (Variables|Default|GetbIsDead)
    (Rendering|SetVisibility (Variables|Default|GetMinimapIcon) false false)
    (Rendering|SetVisibility (Variables|Default|GetWeapon) false false)
    (Collision|SetCollisionEnabled (Variables|Default|GetCapsuleComponent) "NoCollision")))

(fn ConstructionScript)