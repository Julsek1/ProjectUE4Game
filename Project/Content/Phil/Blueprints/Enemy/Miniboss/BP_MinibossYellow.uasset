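; BP_MinibossYellow is an enemy miniboss Blueprint whose own logic mainly manages its minimap icon.
; On BeginPlay it sets the first player character as its owner and tints the MinimapIcon sprite with its Color value.
; Tick polls IsDead every frame and hides the icon once the miniboss is dead.
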(event EventBeginPlay
  (Actor|SetOwner (Game|GetPlayerCharacter 0))
  (Sprite|SetSpriteColor (Variables|Default|GetMinimapIcon) (Math|Conversions|ToLinearColor(Color) (Variables|Default|GetColor))))

(event Collision|EventActorBeginOverlap
  (params (OtherActor :type Actor%20Object%20Reference)))

(event EventTick
  (params (DeltaSeconds :type Float%20%28single-precision%29))
  (if (Variables|Default|GetbIsDead)
    (Rendering|SetVisibility (Variables|Default|GetMinimapIcon) false false)))

(fn ConstructionScript)