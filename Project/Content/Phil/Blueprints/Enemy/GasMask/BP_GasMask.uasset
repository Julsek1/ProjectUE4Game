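; BP_GasMask is a gas mask enemy Blueprint that connects the enemy to its weapon and handles its appearance after death.
; On BeginPlay it sets the player character as its owner and caches the ActiveWeapon child actor as a GasMaskEnemyWeapon.
; Tick polls IsDead and, while true, hides the minimap marker and weapon and disables capsule collision.
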(event EventBeginPlay
  (Actor|SetOwner (Game|GetPlayerCharacter 0))
  (bind _asgas_mask_enemy_weapon (Utilities|Casting|CastToGasMaskEnemyWeapon (Variables|/Script/Engine.ChildActorComponent|GetChildActor (Variables|Default|GetActiveWeapon))))
  (Variables|Default|SetWeapon _asgas_mask_enemy_weapon))

(event Collision|EventActorBeginOverlap
  (params (OtherActor :type Actor%20Object%20Reference)))

(event EventTick
  (params (DeltaSeconds :type Float%20%28single-precision%29))
  (if (Variables|Default|GetbIsDead)
    (Rendering|SetVisibility (Variables|Default|GetMinimapMarker) false false)
    (Rendering|SetVisibility (Variables|Default|GetActiveWeapon) false false)
    (Collision|SetCollisionEnabled (Variables|Default|GetCapsuleComponent) "NoCollision")))

(fn ConstructionScript)