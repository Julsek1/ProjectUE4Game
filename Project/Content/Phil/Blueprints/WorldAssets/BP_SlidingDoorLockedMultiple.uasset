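; BP_SlidingDoorLockedMultiple is a sliding door that opens only once all of its assigned keys are collected.
; A key counts as collected when its entry in the Keys array is no longer valid.
; Trigger overlap by anything other than another door of this class plays a timeline that lerps the Door between Closed and Open positions.
; Leaving the trigger reverses the timeline.
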(event OnComponentBeginOverlap(Trigger)
  (params (OverlappedComponent :type Primitive%20Component%20Object%20Reference) (OtherActor :type Actor%20Object%20Reference) (OtherComp :type Primitive%20Component%20Object%20Reference) (OtherBodyIndex :type Integer) (bFromSweep :type Boolean) (SweepResult :type Hit%20Result%20Structure%20%28by%20ref%29))
  (Utilities|Casting|CastToBP_SlidingDoorLockedMultiple OtherActor
    (:CastFailed
      (bind _keysarecollected (CallFunction|CheckifKeysAreCollected))
      (if _keysarecollected
        (bind _doormovement (Timeline|OpenClose Play)
          (:Update
            (Transformation|SetRelativeLocation (Variables|Default|GetDoor) (Math|Vector|Lerp(Vector) (Variables|Default|GetClosed) (Variables|Default|GetOpen) _doormovement) false false)))))))

(event OnComponentEndOverlap(Trigger)
  (params (OverlappedComponent :type Primitive%20Component%20Object%20Reference) (OtherActor :type Actor%20Object%20Reference) (OtherComp :type Primitive%20Component%20Object%20Reference) (OtherBodyIndex :type Integer))
  (Utilities|Casting|CastToBP_SlidingDoorLockedMultiple OtherActor
    (:CastFailed
      (bind _doormovement (Timeline|OpenClose Reverse)
        (:Update
          (Transformation|SetRelativeLocation (Variables|Default|GetDoor) (Math|Vector|Lerp(Vector) (Variables|Default|GetClosed) (Variables|Default|GetOpen) _doormovement) false false))))))

(fn ConstructionScript)

(fn CheckifKeysAreCollected
  (Variables|Default|SetAllKeysCollected true)
  (bind _array_element (Utilities|Array|ForEachLoopwithBreak (Variables|Default|GetKeys) :!label _label)
    (:LoopBody
      (Utilities|IsValid _array_element
        (:Is%20Valid
          (Variables|Default|SetAllKeysCollected false)
          (goto _label Break))))
    (:Completed
      (return (Variables|Default|GetAllKeysCollected)))))