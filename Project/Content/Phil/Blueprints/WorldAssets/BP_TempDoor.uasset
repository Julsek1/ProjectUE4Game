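; BP_TempDoor is a placeholder door that removes itself when the player's current objective is complete.
; On Tick, while its location differs from FinalPosition, it casts player character 0 to BP_TwinStickShooterPlayer and polls CurrentObjective's Complete flag, then destroys the actor.
; A SetActorLocation to FinalPosition is left unconnected, so the door never moves there.
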(event EventBeginPlay)

(event Collision|EventActorBeginOverlap
  (params (OtherActor :type Actor%20Object%20Reference)))

(event EventTick
  (params (DeltaSeconds :type Float%20%28single-precision%29))
  (if (Math|Vector|NotEqual(Vector) (Transformation|GetActorLocation) (Variables|Default|GetFinalPosition) 0.0001)
    (bind _asbp_twin_stick_shooter_player (Utilities|Casting|CastToBP_TwinStickShooterPlayer (Game|GetPlayerCharacter 0)))
    (if (Variables|/Script/Project.Objective|GetbComplete (Variables|/Script/Project.TwinStickShooterPlayer|GetCurrentObjective _asbp_twin_stick_shooter_player))
      (Actor|DestroyActor))))

(fn ConstructionScript)