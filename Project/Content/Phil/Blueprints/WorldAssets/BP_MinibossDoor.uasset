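; Door actor tied to a Miniboss that teleports the player to a set location while that miniboss still exists.
; On BeginPlay it creates a dynamic material on the Door and tints it with the miniboss's color.
; Any actor overlap teleports player 0 to TeleportLocation, keeping their rotation, if the Miniboss reference is valid.
; Tick polls that reference and turns the door black once it is invalid, when overlaps no longer teleport.
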(event EventBeginPlay
  (bind _returnvalue (Rendering|Material|CreateDynamicMaterialInstance (Variables|Default|GetDoor) 0 0 "None" :!class /Script/Engine.PrimitiveComponent))
  (bind _output_get (Variables|Default|SetMaterialInstance _returnvalue))
  (Rendering|Material|SetVectorParameterValue _output_get "MaterialColor" (Math|Conversions|ToLinearColor(Color) (Variables|/Script/Project.Miniboss|GetColor (Variables|Default|GetMiniboss))) :!class /Script/Engine.MaterialInstanceDynamic))

(event Collision|EventActorBeginOverlap
  (params (OtherActor :type Actor%20Object%20Reference))
  (bind _returnvalue (Game|GetPlayerCharacter 0))
  (Utilities|IsValid (Variables|Default|GetMiniboss)
    (:Is%20Valid
      (Transformation|Teleport _returnvalue (Variables|Default|GetTeleportLocation) (Transformation|GetActorRotation _returnvalue)))))

(event EventTick
  (params (DeltaSeconds :type Float%20%28single-precision%29))
  (Utilities|IsValid (Variables|Default|GetMiniboss)
    (:Is%20Not%20Valid
      (Rendering|Material|SetVectorParameterValue (Variables|Default|GetMaterialInstance) "MaterialColor" (Class|KismetMathLibrary|LinearColorBlack) :!class /Script/Engine.MaterialInstanceDynamic))))

(fn ConstructionScript)