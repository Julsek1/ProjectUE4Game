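; BP_MinibossDoorMultiple is a door that unlocks as a teleporter once two referenced minibosses are gone.
; Tick polls both references and, when neither is valid, sets the BossIsDead material parameter on the Door every frame.
; In that state, it also checks whether player character 0 overlaps the Collider and teleports them to TeleportLocation, keeping their rotation.
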(event EventBeginPlay)

(event Collision|EventActorBeginOverlap
  (params (OtherActor :type Actor%20Object%20Reference)))

(event EventTick
  (params (DeltaSeconds :type Float%20%28single-precision%29))
  (bind _returnvalue (Game|GetPlayerCharacter 0))
  (Utilities|IsValid (Variables|Default|GetMiniboss)
    (:Is%20Not%20Valid
      (Utilities|IsValid (Variables|Default|GetMiniboss2)
        (:Is%20Not%20Valid
          (Rendering|Material|SetScalarParameterValueonMaterials (Variables|Default|GetDoor) "BossIsDead" 1.0)
          (if (Collision|IsOverlappingActor (Variables|Default|GetCollider) (Game|GetPlayerCharacter 0) :!class /Script/Engine.PrimitiveComponent)
            (Transformation|Teleport _returnvalue (Variables|Default|GetTeleportLocation) (Transformation|GetActorRotation _returnvalue))))))))

(fn ConstructionScript)