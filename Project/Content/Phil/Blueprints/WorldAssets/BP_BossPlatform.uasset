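; BP_BossPlatform is a boss platform that collapses once explosives are planted on all four of its pillars.
; Tick polls the ExplosivePlanted flag on the first four entries of the Pillars array until all are true, then sets Destroyed.
; On a later tick, a DoOnce calls ExplodePillars, which enables physics simulation on the platform's static mesh and calls Explode on every pillar.
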(event EventBeginPlay)

(event Collision|EventActorBeginOverlap
  (params (OtherActor :type Actor%20Object%20Reference)))

(event EventTick
  (params (DeltaSeconds :type Float%20%28single-precision%29))
  (bind _pillars (Variables|Default|GetPillars))
  (if (Variables|Default|GetDestroyed)
    (Utilities|FlowControl|DoOnce false
      (:Completed
        (CallFunction|ExplodePillars)))
    (else
      (Variables|Default|SetDestroyed (Math|Boolean|ANDBoolean (Variables|/Script/Project.MinibossLevelPillar|GetbExplosivePlanted (Utilities|Array|Get(acopy) _pillars)) (Variables|/Script/Project.MinibossLevelPillar|GetbExplosivePlanted (Utilities|Array|Get(acopy) _pillars 1)) (Variables|/Script/Project.MinibossLevelPillar|GetbExplosivePlanted (Utilities|Array|Get(acopy) _pillars 2)) (Variables|/Script/Project.MinibossLevelPillar|GetbExplosivePlanted (Utilities|Array|Get(acopy) _pillars 3)))))))

(fn ConstructionScript)

(fn ExplodePillars
  (Physics|SetSimulatePhysics (Variables|Default|GetStaticMesh) true)
  (for _array_element (Variables|Default|GetPillars)
    (Class|MinibossLevelPillar|Explode _array_element)))