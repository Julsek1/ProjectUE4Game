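; BP_ServerRoomSpawner releases waves of pre-placed enemies while the player hacks server room terminals.
; Enemies' widgets are hidden on BeginPlay.
; Tick watches each interacted terminal's hack timer and, at each breakpoint, advances it by SpawnRate and moves the next unused enemies to the spawn Locations.
; Moved enemies get their widgets shown and the player's current location written to their gas mask AI controller's blackboard.
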(event EventBeginPlay
  (for _array_element (Variables|Default|GetEnemies)
    (Rendering|SetVisibility (Variables|/Script/Project.ParentEnemy|GetWidgetComponent _array_element) false false)))

(event Collision|EventActorBeginOverlap
  (params (OtherActor :type Actor%20Object%20Reference)))

(event EventTick
  (params (DeltaSeconds :type Float%20%28single-precision%29))
  (bind _enemies (Variables|Default|GetEnemies))
  (bind _index (Variables|Default|GetIndex))
  (bind _terminalbreakpoint (Variables|Default|GetTerminalBreakpoint))
  (bind _output (Utilities|Array|Get(acopy) _enemies _index))
  (for (_array_element _array_index) (Variables|Default|GetTerminals)
    (Utilities|IsValid _array_element
      (:Is%20Valid
        (if (and (>= (Class|KismetSystemLibrary|GetTimerElapsedTimeHandle (Variables|/Script/Project.InteractableTerminal|GetHackTimerHandle _array_element)) (Utilities|Array|Get(acopy) (Variables|Default|GetTerminalBreakpoint) _array_index)) (Variables|/Script/Project.InteractableActor|GetbHasBeenInteractedWith _array_element))
          (Utilities|Array|SetArrayElem _terminalbreakpoint _array_index (+ (Utilities|Array|Get(acopy) _terminalbreakpoint _array_index) (Variables|Default|GetSpawnRate)))
          (for _array_element_2 (Variables|Default|GetLocations)
            (Transformation|SetActorLocation _output (Transformation|GetActorLocation _array_element_2) false false)
            (Rendering|SetVisibility (Variables|/Script/Project.ParentEnemy|GetWidgetComponent _output) true false)
            (bind _asaic_gas_mask_enemy (Utilities|Casting|CastToAIC_GasMaskEnemy (AI|GetAIController _output)))
            (AI|Components|Blackboard|SetValueasVector (Variables|/Script/AIModule.AIController|GetBlackboard _asaic_gas_mask_enemy) (Variables|/Game/Phil/AI/GasMask/AIC_GasMaskEnemy.AIC_GasMaskEnemy_C|GetPlayerLocationKey _asaic_gas_mask_enemy) (Transformation|GetActorLocation (Game|GetPlayerCharacter 0)))
            (Math|Integer|IncrementInt (Variables|Default|GetIndex))))))))

(fn ConstructionScript)