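; BP_InteractableTerminal is an interactable world terminal that displays a hack progress widget once it has been interacted with.
; On BeginPlay it hands itself to the TSHackWidget inside its HackProgress component, then hides that component.
; Tick polls the HasBeenInteractedWith flag and makes the component visible while it is true.
; Nothing in these graphs sets the flag or hides the widget again.
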(event EventBeginPlay
  (bind _astshack_widget (Utilities|Casting|CastToTSHackWidget (UserInterface|GetUserWidgetObject (Variables|Default|GetHackProgress))))
  (Variables|/Script/Project.TSHackWidget|SetTerminal _astshack_widget self)
  (Rendering|SetVisibility (Variables|Default|GetHackProgress) false false))

(event Collision|EventActorBeginOverlap
  (params (OtherActor :type Actor%20Object%20Reference)))

(event EventTick
  (params (DeltaSeconds :type Float%20%28single-precision%29))
  (if (Variables|Default|GetbHasBeenInteractedWith)
    (Rendering|SetVisibility (Variables|Default|GetHackProgress) true false)))

(fn ConstructionScript)