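; BP_ToggleableDoors is a door actor that switches between a solid, visible state and a hidden, passable one.
; Its Toggle function checks whether the static mesh has collision enabled, then flips both collision and visibility to the opposite state, with no animation.
; BeginPlay calls Toggle once, so each door starts play in the inverse of its configured collision state.
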(event EventBeginPlay
  (CallFunction|Toggle))

(event Collision|EventActorBeginOverlap
  (params (OtherActor :type Actor%20Object%20Reference)))

(event EventTick
  (params (DeltaSeconds :type Float%20%28single-precision%29)))

(fn ConstructionScript)

(fn Toggle
  (bind _staticmesh (Variables|Default|GetStaticMesh))
  (bind _staticmesh_2 (Variables|Default|GetStaticMesh))
  (if (Class|PrimitiveComponent|IsCollisionEnabled (Variables|Default|GetStaticMesh))
    (Collision|SetCollisionEnabled _staticmesh_2 "NoCollision")
    (Rendering|SetVisibility _staticmesh false false)
    (else
      (Collision|SetCollisionEnabled _staticmesh_2 "QueryAndPhysics")
      (Rendering|SetVisibility _staticmesh true false))))