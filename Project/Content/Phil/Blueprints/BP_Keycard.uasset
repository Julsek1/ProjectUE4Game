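; BP_Keycard is a keycard actor that spins in the world and is kept off the player's minimap.
; On BeginPlay it casts the player character to BP_TwinStickShooterPlayer and adds itself to the MinimapCapture2D hidden actors.
; Tick rotates the Collider component around yaw at a constant, frame-rate-independent speed.
; The Blueprint's graphs contain no pickup or overlap logic.
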(event EventBeginPlay
  (bind _asbp_twin_stick_shooter_player (Utilities|Casting|CastToBP_TwinStickShooterPlayer (Game|GetPlayerCharacter 0)))
  (Utilities|Array|Add (Variables|/Script/Engine.SceneCaptureComponent|GetHiddenActors (Variables|/Game/Phil/Blueprints/BP_TwinStickShooterPlayer.BP_TwinStickShooterPlayer_C|GetMinimapCapture2D _asbp_twin_stick_shooter_player)) self))

(event Collision|EventActorBeginOverlap
  (params (OtherActor :type Actor%20Object%20Reference)))

(event EventTick
  (params (DeltaSeconds :type Float%20%28single-precision%29))
  (bind _collider (Variables|Default|GetCollider))
  (bind _returnvalue (Transformation|GetWorldRotation _collider))
  (Transformation|SetWorldRotation _collider (Math|Rotator|MakeRotator (.roll _returnvalue) (.pitch _returnvalue) (+ (.yaw _returnvalue) (* 50 DeltaSeconds))) false false))

(fn ConstructionScript)