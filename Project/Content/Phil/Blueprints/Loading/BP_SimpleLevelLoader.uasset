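; Level-transition actor that opens a named level after a short delay when the player overlaps it, carrying the collectible count across levels.
; On BeginPlay it restores the count from a BP_CollectiblesSaveGame slot or creates one, then binds saving to the twin-stick player's save dispatcher.
; It saves on overlap and on that event.
; EndPlay zeroes the saved count unless a level load started or Tick saw the player's health reach zero.
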(event Custom|SaveCollectibleEvent
  (CallFunction|SaveCollectibles))

(event EventBeginPlay
  (Utilities|FlowControl|Sequence
    (:then_0
      (bind _asparent_player (Utilities|Casting|CastToParentPlayer (Game|GetPlayerCharacter 0)))
      (Variables|Default|SetPlayer _asparent_player)
      (bind _returnvalue (SaveGame|DoesSaveGameExist (Variables|Default|GetSlot)))
      (if _returnvalue
        (bind _returnvalue_2 (SaveGame|LoadGamefromSlot (Variables|Default|GetSlot)))
        (bind _asbp_collectibles_save_game (Utilities|Casting|CastToBP_CollectiblesSaveGame _returnvalue_2))
        (bind _output_get (Variables|Default|SetSaverSubclass _asbp_collectibles_save_game))
        (Variables|/Script/Project.ParentPlayer|SetNumberOfCollectibles (Variables|Default|GetPlayer) (Variables|/Game/Phil/Blueprints/Saving/BP_CollectiblesSaveGame.BP_CollectiblesSaveGame_C|GetCollectibles _output_get))
        (SaveGame|SaveGametoSlot (Variables|Default|GetSaverSubclass) (Variables|Default|GetSlot))
        (else
          (bind _returnvalue_3 (SaveGame|CreateSaveGameObject "/Game/Phil/Blueprints/Saving/BP_CollectiblesSaveGame.BP_CollectiblesSaveGame_C"))
          (bind _output_get_2 (Variables|Default|SetSaverSubclass _returnvalue_3))
          (Variables|/Game/Phil/Blueprints/Saving/BP_CollectiblesSaveGame.BP_CollectiblesSaveGame_C|SetCollectibles _output_get_2 0)
          (SaveGame|SaveGametoSlot (Variables|Default|GetSaverSubclass) (Variables|Default|GetSlot)))))
    (:then_1
      (bind _asbp_twin_stick_shooter_player (Utilities|Casting|CastToBP_TwinStickShooterPlayer (Variables|Default|GetPlayer)))
      (EventDispatchers|BindEventtoSaveEventDispatcher _asbp_twin_stick_shooter_player (delegate Custom|SaveCollectibleEvent)))))

(event Collision|EventActorBeginOverlap
  (params (OtherActor :type Actor%20Object%20Reference))
  (Utilities|Casting|CastToParentPlayer OtherActor)
  (Variables|Default|SetLoading true)
  (CallFunction|SaveCollectibles)
  (Utilities|FlowControl|Delay 0.5)
  (Game|OpenLevel(byName) (Variables|Default|GetLevelName)))

(event EventTick
  (params (DeltaSeconds :type Float%20%28single-precision%29))
  (bind _player (Variables|Default|GetPlayer))
  (Utilities|IsValid _player
    (:Is%20Valid
      (if (<= (Variables|/Script/Project.ParentPlayer|GetHealth _player) 0.0)
        (Variables|Default|SetPlayerDead true)))))

(event EventEndPlay
  (params (EndPlayReason :type EEndPlayReason%20Enum :default "Destroyed"))
  (if (and (not (Variables|Default|GetLoading)) (not (Variables|Default|GetPlayerDead)))
    (Variables|/Game/Phil/Blueprints/Saving/BP_CollectiblesSaveGame.BP_CollectiblesSaveGame_C|SetCollectibles (Variables|Default|GetSaverSubclass) 0)
    (SaveGame|SaveGametoSlot (Variables|Default|GetSaverSubclass) (Variables|Default|GetSlot))))

(fn ConstructionScript)

(fn SaveCollectibles
  (Variables|/Game/Phil/Blueprints/Saving/BP_CollectiblesSaveGame.BP_CollectiblesSaveGame_C|SetCollectibles (Variables|Default|GetSaverSubclass) (Variables|/Script/Project.ParentPlayer|GetNumberOfCollectibles (Variables|Default|GetPlayer)))
  (SaveGame|SaveGametoSlot (Variables|Default|GetSaverSubclass) (Variables|Default|GetSlot)))