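; Mutant enemy NPC character with health-based death and a melee attack animation.
; Tick prints Hp for debugging and, once it reaches zero, plays the dying animation a single time and flags IsDeseased.
; Death also sets IsDead on the AI Blackboard, disables capsule collision and destroys the actor after a delay.
; The MeleeAttack event only plays the attack montage on the mesh, with no damage logic here.
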(event EventBeginPlay)

(event Collision|EventActorBeginOverlap
  (params (OtherActor :type Actor%20Object%20Reference)))

(event EventTick
  (params (DeltaSeconds :type Float%20%28single-precision%29))
  (Development|PrintString (Utilities|String|ToString(Float) (Variables|Default|GetHp)))
  (if (<= (Variables|Default|GetHp) 0.0)
    (if (not (Variables|Default|GetIsDeseased))
      (Components|Animation|PlayAnimation (Variables|Character|GetMesh) "/Game/Julian/Enemies/NPCMutant/NPCMutantAnimations/Mutant2_Dying.Mutant2_Dying" false)
      (bind _output_get (Variables|Default|SetIsDeseased true))
      (AI|Components|Blackboard|SetValueasBool (AI|GetBlackboard 0) (Utilities|Name|MakeLiteralName "IsDead") _output_get)
      (Collision|SetCollisionEnabled (Variables|Default|GetCapsuleComponent) "NoCollision")
      (Utilities|FlowControl|Delay 8.0)
      (Actor|DestroyActor))))

(event EventMeleeAttack
  (Animation|Montage|PlayMontage (Variables|Character|GetMesh) "/Game/Julian/Enemies/NPCMutant/NPCMutantAnimations/NPCAttack_AnimMontage.NPCAttack_AnimMontage"))

(fn ConstructionScript)