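; Gas mask enemy Blueprint that reacts to gun hits and signals when it has detected the player.
; BeginPlay sets the player character as owner and caches the weapon from its child actor.
; Overlapping a Gun triggers hit animation, light damage, effects, then delayed detection.
; Tick briefly shows a player-facing alert upon detection; its death cleanup of marker, weapon and collision sits inside the not-dead check.
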(event EventBeginPlay
  (Actor|SetOwner (Game|GetPlayerCharacter 0))
  (bind _asgas_mask_enemy_weapon (Utilities|Casting|CastToGasMaskEnemyWeapon (Variables|/Script/Engine.ChildActorComponent|GetChildActor (Variables|Default|GetActiveWeapon))))
  (Variables|Default|SetWeapon _asgas_mask_enemy_weapon))

(event Collision|EventActorBeginOverlap
  (params (OtherActor :type Actor%20Object%20Reference))
  (bind _asgun (Utilities|Casting|CastToGun OtherActor))
  (Components|Animation|PlayAnimation (Variables|Character|GetMesh) "/Game/Julian/Enemies/JGasMask/Hit_Reaction.Hit_Reaction" false)
  (Class|ParentEnemy|GetHit 0.2 0.0 "0.000000,0.000000,0.000000")
  (Effects|SpawnEmitteratLocation "/Game/MilitaryWeapDark/FX/P_Impact_Stone_Large_01.P_Impact_Stone_Large_01" (Transformation|GetActorLocation _asgun))
  (Audio|PlaySoundatLocation "/Game/MilitaryWeapDark/Sound/Knife/Knife_ImpactBody_Cue.Knife_ImpactBody_Cue" (Transformation|GetActorLocation _asgun) "0, 0, 0" 1.0 1.0 0.0 0 0 0)
  (Utilities|FlowControl|Delay 1.0)
  (Variables|Default|SetbDetectedPlayer true))

(event EventTick
  (params (DeltaSeconds :type Float%20%28single-precision%29))
  (if (not (Variables|Default|GetbIsDead))
    (if (Variables|Default|GetbDetectedPlayer)
      (Rendering|SetVisibility (Variables|Default|GetAlert) true false)
      (Transformation|SetWorldRotation (Variables|Default|GetAlert) (Math|Rotator|FindLookatRotation (Transformation|GetActorLocation) (Transformation|GetActorLocation (Game|GetPlayerCharacter 0))) false false)
      (Utilities|FlowControl|Delay 1.5)
      (Rendering|SetVisibility (Variables|Default|GetAlert) false false))
    (if (Variables|Default|GetbIsDead)
      (Rendering|SetVisibility (Variables|Default|GetMinimapMarker) false false)
      (Rendering|SetVisibility (Variables|Default|GetActiveWeapon) false false)
      (Collision|SetCollisionEnabled (Variables|Default|GetCapsuleComponent) "NoCollision"))))

(fn ConstructionScript)