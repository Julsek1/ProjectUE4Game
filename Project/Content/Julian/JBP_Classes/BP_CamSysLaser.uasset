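; BP_CamSysLaser is a trigger-driven camera actor that takes over the player's view in part of a level.
; StartCamera overlap blends the view to this actor and records the spring arm's offset from the player once; EndCamera overlap blends back to the player.
; While it is the view target, Tick either rotates a static camera toward the player or repositions the spring arm through VInterpTo, using TrackChar as a per-axis follow mask.
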(event OnComponentBeginOverlap(StartCamera)
  (params (OverlappedComponent :type Primitive%20Component%20Object%20Reference) (OtherActor :type Actor%20Object%20Reference) (OtherComp :type Primitive%20Component%20Object%20Reference) (OtherBodyIndex :type Integer) (bFromSweep :type Boolean) (SweepResult :type Hit%20Result%20Structure%20%28by%20ref%29))
  (Utilities|Casting|CastToJBasePlayer OtherActor)
  (Game|Player|SetViewTargetwithBlend (Game|GetPlayerController 0) self (Variables|Default|GetBlendTime) "VTBlend_Linear" 0.0 false)
  (Utilities|FlowControl|DoOnce false
    (:Completed
      (Variables|Default|SetOffSet (- (Transformation|GetWorldLocation (Variables|Default|GetSpringArm)) (Transformation|GetActorLocation (Game|GetPlayerCharacter 0)))))))

(event OnComponentBeginOverlap(EndCamera)
  (params (OverlappedComponent :type Primitive%20Component%20Object%20Reference) (OtherActor :type Actor%20Object%20Reference) (OtherComp :type Primitive%20Component%20Object%20Reference) (OtherBodyIndex :type Integer) (bFromSweep :type Boolean) (SweepResult :type Hit%20Result%20Structure%20%28by%20ref%29))
  (bind _asjbase_player (Utilities|Casting|CastToJBasePlayer OtherActor))
  (Game|Player|SetViewTargetwithBlend (Game|GetPlayerController 0) _asjbase_player (Variables|Default|GetBlendTime) "VTBlend_Linear" 0.0 false))

(event EventTick
  (params (DeltaSeconds :type Float%20%28single-precision%29))
  (if (== (Pawn|GetViewTarget (Game|GetPlayerController 0)) self)
    (if (Variables|Default|GetIsStatic)
      (bind _rotation (CallFunction|TrackCharRotation DeltaSeconds))
      (Transformation|SetWorldRotation (Variables|Default|GetCamera) _rotation false false)
      (else
        (bind _vector (CallFunction|TrackCharMov DeltaSeconds))
        (Transformation|SetWorldLocation (Variables|Default|GetSpringArm) _vector false false)))))

(fn ConstructionScript)

(fn TrackCharMov
  (params (DeltaTime :type Float%20%28single-precision%29))
  (bind _returnvalue (Transformation|GetActorLocation))
  (bind _offset (Variables|Default|GetOffSet))
  (bind _trackchar (Variables|Default|GetTrackChar))
  (bind _returnvalue_2 (- _returnvalue _offset))
  (return (Math|Interpolation|VInterpTo _returnvalue_2 (+ (* (Transformation|GetActorLocation (Game|GetPlayerCharacter 0)) _trackchar) (* _returnvalue_2 (- "1.000000,1.000000,1.000000" _trackchar))) DeltaTime 0.0)))

(fn TrackCharRotation
  (params (DeltaTime :type Float%20%28single-precision%29))
  (return (Math|Rotator|FindLookatRotation (Transformation|GetWorldLocation (Variables|Default|GetCamera)) (Transformation|GetActorLocation (Game|GetPlayerCharacter 0)))))