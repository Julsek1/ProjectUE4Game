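; Game mode Blueprint meant to run a mission countdown that prints a failure message and reloads the current level at zero.
; Tick holds the timer, using a one-second Delay to decrement Seconds and Minutes, behind two branches apparently intended to skip ending levels.
; The level-name comparisons are unwired and the first branch is constantly true, so Tick only removes all widgets and never reaches the countdown.
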(event EventBeginPlay)

(event EventTick
  (params (DeltaSeconds :type Float%20%28single-precision%29))
  (bind _returnvalue (Game|GetCurrentLevelName true))
  (if true
    (Viewport|RemoveAllWidgets)
    (else
      (bind _returnvalue_2 (Game|GetCurrentLevelName true))
      (if true
        (Viewport|RemoveAllWidgets)
        (else
          (Utilities|FlowControl|Delay 1.0)
          (Variables|Default|SetSeconds (- (Variables|Default|GetSeconds) 1))
          (if (< (Variables|Default|GetSeconds) 0)
            (Variables|Default|SetMinutes (- (Variables|Default|GetMinutes) 1))
            (Variables|Default|SetSeconds 59))
          (if (== (Variables|Default|GetSeconds) 0)
            (if (== (Variables|Default|GetMinutes) 0)
              (Development|PrintString "Mision Failed" true true "(R=1.000000,G=1.000000,B=1.000000,A=0.882000)")
              (Utilities|FlowControl|Delay 1.0)
              (bind _returnvalue_3 (Game|GetCurrentLevelName true))
              (Game|OpenLevel(byName) (Utilities|String|StringToName _returnvalue_3)))))))))

(fn ConstructionScript)